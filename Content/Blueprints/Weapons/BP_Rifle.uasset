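; BP_Rifle is an automatic rifle weapon that keeps firing from StartShooting until StopShooting.
; StartShooting fires immediately, plays the gun mesh's fire animation, and starts a looping timer at the FireRate interval.
; Each timer tick repeats FireWeapon and the animation through the fireRifle event, and StopShooting clears the stored timer handle.
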(event Custom|fireRifle
  (CallFunction|FireWeapon)
  (Components|Animation|PlayAnimation (Variables|Default|GetGunMesh) "/Game/MilitaryWeapSilver/Weapons/Animations/Fire_Rifle_W.Fire_Rifle_W" false))

(event EventBeginPlay
  (|CallParentFunction) ; This node is disabled and will not be called.\nDrag off pins to build functionality.
)

(event Collision|EventActorBeginOverlap
  (params (OtherActor :type Actor%20Object%20Reference))
  (|CallParentFunction OtherActor) ; This node is disabled and will not be called.\nDrag off pins to build functionality.
)

(event EventTick
  (params (DeltaSeconds :type Float%20%28single-precision%29))
  (|CallParentFunction DeltaSeconds) ; This node is disabled and will not be called.\nDrag off pins to build functionality.
)

(event EventStartShooting
  (CallFunction|FireWeapon)
  (Components|Animation|PlayAnimation (Variables|Default|GetGunMesh) "/Game/MilitaryWeapSilver/Weapons/Animations/Fire_Rifle_W.Fire_Rifle_W" false)
  (bind _returnvalue (Utilities|Time|SetTimerbyEvent (delegate Custom|fireRifle) (Variables|Default|GetfireRate) true))
  (Variables|Default|SetfireEvent _returnvalue))

(event EventStopShooting
  (Utilities|Time|ClearandInvalidateTimerbyHandle (Variables|Default|GetfireEvent)))

(fn ConstructionScript
  (|CallParentFunction))